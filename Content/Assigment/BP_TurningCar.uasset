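; BP_TurningCar is an actor that spins continuously in the world and can be removed with a mouse click.
; Tick adds a rotation offset to the actor's world rotation each frame, independent of delta time.
; BeginPlay enables input through player controller 0, so any left mouse press destroys the actor and prints a greeting.
; An unconnected debug print of the current rotation is left in the graph.
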(event EventTick
  (params (DeltaSeconds :type Float%20%28single-precision%29))
  (Class|Actor|AddActorWorldRotation (Variables|Default|GetRotationToAdd)))

(event EventBeginPlay
  (Input|EnableInput (Game|GetPlayerController 0) 0))

(event Input|MouseEvents|LeftMouseButton
  (params (Key :type Key%20Structure :default "None"))
  (:Pressed
    (Actor|DestroyActor)
    (Development|PrintString "Hello")))

(fn ConstructionScript)