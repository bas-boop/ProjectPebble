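; BP_MyFirstBlueprint is a simple Blueprint that either deletes a referenced actor or attempts a spawn, printing a message either way.
; BeginPlay and a custom Yes event share one chain, which runs only when OtherActor is valid.
; ShouldDelete selects between destroying OtherActor and calling SpawnActor at a fixed transform, though the spawn class is left empty.
; Each message joins the actor's display name with that branch's string variable.
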(event Custom|Yes
  (bind _otheractor (Variables|Default|GetOtherActor)
    (:then
      (if (Variables|Default|GetShouldDelete)
        (Development|PrintString (Utilities|String|Append (Utilities|GetDisplayName _otheractor) (Variables|Default|GetStringToDelete)))
        (Actor|DestroyActor (Variables|Default|GetOtherActor))
        (else
          (Development|PrintString (Utilities|String|Append (Utilities|GetDisplayName _otheractor) (Variables|Default|GetStringToSpawn)))
          (Game|SpawnActorfromClass "/Game/Empty.Empty_C" (Math|Transform|MakeTransform "-200.000000,0.000000,100.000000") "Undefined" "MultiplyWithRoot" 0 0))))
    (:else)))

(event EventBeginPlay
  (bind _otheractor (Variables|Default|GetOtherActor)
    (:then
      (if (Variables|Default|GetShouldDelete)
        (Development|PrintString (Utilities|String|Append (Utilities|GetDisplayName _otheractor) (Variables|Default|GetStringToDelete)))
        (Actor|DestroyActor (Variables|Default|GetOtherActor))
        (else
          (Development|PrintString (Utilities|String|Append (Utilities|GetDisplayName _otheractor) (Variables|Default|GetStringToSpawn)))
          (Game|SpawnActorfromClass "/Game/Empty.Empty_C" (Math|Transform|MakeTransform "-200.000000,0.000000,100.000000") "Undefined" "MultiplyWithRoot" 0 0))))
    (:else)))

(fn ConstructionScript)