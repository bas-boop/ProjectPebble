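; BP_EntityStateMachine is an entity Blueprint that sets up a component-based state machine with idle and walk states.
; On BeginPlay, it checks that both state components are valid, then packs them into the shared data struct on BPCStateMachine.
; It then initializes the state machine with a state array in which only the idle and walk slots are filled.
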(event EventBeginPlay
  (bind _bpc_idlestate (Variables|Default|GetBPC_IdleState))
  (bind _bpc_walkstate (Variables|Default|GetBPC_WalkState))
  (Utilities|IsValid _bpc_idlestate
    (:Is%20Valid
      (Utilities|IsValid _bpc_walkstate
        (:Is%20Valid
          (Variables|/Game/StateSystem/BPC_StateMachine.BPC_StateMachine_C|SetSharedData (Variables|Default|GetBPC_StateMachine) (Utilities|Struct|MakeS_SharedData _bpc_idlestate _bpc_walkstate))
          (bind _output_get (Variables|Default|SetStates (Utilities|Array|MakeArray (Variables|Default|GetBPC_IdleState) (Variables|Default|GetBPC_WalkState) 0 0 0 0 0 0 0 0 0)))
          (Default|INit (Variables|Default|GetBPC_StateMachine) _output_get))))))

(fn ConstructionScript)